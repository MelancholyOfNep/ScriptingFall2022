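; TriggerScore is an overlap trigger actor that awards score through the BouncyRoom game mode.
; When any actor begins overlapping it, it casts the game mode to BouncyRoom, adds one point and spawns a Sparks particle system at that actor's location.
; It also prints the actor's name on entry, only if the cast succeeds, and on exit.
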(event `self.ReceiveActorBeginOverlap`
  (params (OtherActor :type "Actor Object Reference"))
  (bind _asbouncy_room (cast `/Game/Blueprints/BouncyRoom` (`GameplayStatics.GetGameMode`)))
  (`/Game/Blueprints/BouncyRoom.Add Score` _asbouncy_room 1)
  (`NiagaraFunctionLibrary.SpawnSystemAtLocation` "/Game/Sparks_System.Sparks_System" (`self.K2_GetActorLocation` OtherActor))
  ;[1 1 1] Comment
  (`KismetSystemLibrary.PrintString` (`KismetStringLibrary.Concat_StrStr` (`KismetSystemLibrary.GetDisplayName` OtherActor) "Entered")))

(event `self.ReceiveActorEndOverlap`
  (params (OtherActor :type "Actor Object Reference"))
  (`KismetSystemLibrary.PrintString` (`KismetStringLibrary.Concat_StrStr` (`KismetSystemLibrary.GetDisplayName` OtherActor) "Exited")))

(fn `UserConstructionScript`)